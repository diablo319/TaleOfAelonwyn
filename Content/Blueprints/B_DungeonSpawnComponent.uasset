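; Component on B_DungeonGen that scatters a set quantity of actors from a weighted SpawnList across dungeon floor tiles on BeginPlay.
; It draws random room tiles, plus corridors unless RoomOnly, from the dungeon's seeded stream, rerolling any within MinDistance of the previous spawn only.
; SpawnList classes roll in key order; the first success spawns at the scaled, offset tile, which leaves the pool.
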(event Custom|TriggerSpawnEvent
  (bind _asb_dungeon_gen (Utilities|Casting|CastToB_DungeonGen (Components|GetOwner)))
  (Variables|Default|SetDungeonREF _asb_dungeon_gen)
  (if (Variables|Default|GetRoomOnly)
    (Variables|Default|SetFloorTiles (Variables|/Game/Blueprints/B_DungeonGen.B_DungeonGen_C|GetFloorTiles_RoomOnly (Variables|Default|GetDungeonREF)))
    (else
      (Variables|Default|SetFloorTiles (Variables|/Game/Blueprints/B_DungeonGen.B_DungeonGen_C|GetFloorTiles_RoomOnly (Variables|Default|GetDungeonREF)))
      (Utilities|Array|AppendArray (Variables|Default|GetFloorTiles) (Variables|/Game/Blueprints/B_DungeonGen.B_DungeonGen_C|GetCorridorTiles (Variables|Default|GetDungeonREF)))))
  (CallFunction|SpawnItems))

(event EventBeginPlay
  (CallFunction|TriggerSpawnEvent))

(fn SpawnItems
  (bind _spawnlist (Variables|Default|GetSpawnList))
  (bind _dungeonref (Variables|Default|GetDungeonREF))
  ;[1 1 1] While spawns are less than desired quantity loop spawn logic
  (while (> (Variables|Default|GetQuantity) (LocalVariables|GetItemsSpawned))
    ;[1 1 1] Get random floor tile, test minimum distance
    (bind _output_get (LocalVariables|SetFloorIndex (Math|Random|RandomIntegerinRangefromStream (Variables|/Game/Blueprints/B_DungeonGen.B_DungeonGen_C|GetStream (Variables|Default|GetDungeonREF)) 0 (Utilities|Array|LastIndex (Variables|Default|GetFloorTiles))) :!label _label))
    (|TestMinDistanceBetweenConsecutiveSpawns_2 _output_get
      (:Fail
        (goto _label))
      (:Pass
        ;[1 1 1] Loop through spawn list, if item spawn is true stop looping
        (bind _keys (Utilities|Map|Keys _spawnlist))
        (bind _array_element (Utilities|Array|ForEachLoopwithBreak _keys :!label _label_2)
          (:LoopBody
            (if (Class|KismetMathLibrary|RandomBoolwithWeightfromStream (Variables|/Game/Blueprints/B_DungeonGen.B_DungeonGen_C|GetStream (Variables|Default|GetDungeonREF)) (.Value (Utilities|Map|Find _spawnlist _array_element)))
              (Utilities|FlowControl|Sequence
                (:then_0
                  ;[1 1 1] Spawn actor, save previous location, remove tile from list and increment items spawned
                  (Game|SpawnActorfromClass _array_element (Math|Conversions|ToTransform(Vector) (+ (* (Math|Conversions|ToVector(Float) (Utilities|Array|Get(acopy) (Variables|Default|GetFloorTiles) (LocalVariables|GetFloorIndex))) (Variables|/Game/Blueprints/B_DungeonGen.B_DungeonGen_C|GetScale _dungeonref)) (Transformation|GetActorLocation _dungeonref) (Variables|Default|GetOffset))) "Undefined" "MultiplyWithRoot" 0 0)
                  (LocalVariables|SetLastLocation (* (Math|Conversions|ToVector(Float) (Utilities|Array|Get(acopy) (Variables|Default|GetFloorTiles) (LocalVariables|GetFloorIndex))) (Variables|/Game/Blueprints/B_DungeonGen.B_DungeonGen_C|GetScale _dungeonref)))
                  (Utilities|Array|RemoveIndex (Variables|Default|GetFloorTiles) (LocalVariables|GetFloorIndex))
                  (Math|Integer|IncrementInt (LocalVariables|GetItemsSpawned)))
                (:then_1
                  (goto _label_2 Break))))))))))